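; Game instance that carries state across the Day_Cycle to Night_Cycle level switch and handles restarts.
; Init sets the day flag from the level name and creates the item bar and option widgets.
; ChangeLevel, during day only, stores medicine and item hidden states, has the item bar and AI save themselves, then opens night.
; Restart recreates the item bar, clears the AI death flags and reopens day, without setting IsDay back.
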(event `self.ReceiveInit`
  (bind _returnvalue (`GameplayStatics.GetPlayerController` 0))
  (bind _returnvalue_2 (`GameplayStatics.GetCurrentLevelName` true))
  (`KismetSystemLibrary.PrintString` _returnvalue_2)
  (if (`KismetStringLibrary.EqualEqual_StrStr` _returnvalue_2 "Night_Cycle")
    (set `self.IsDay` false))
  (bind _returnvalue_3 (`|CreateWidget` "/Game/UI/ItemBarUI.ItemBarUI_C" _returnvalue))
  (set `self.ItemBar` _returnvalue_3)
  (bind _returnvalue_4 (`|CreateWidget` "/Game/UI/OptionUI.OptionUI_C" _returnvalue))
  (set `self.OptionUI` _returnvalue_4))

(event `ChangeLevel`
  (bind _playerref (`self.PlayerRef`))
  (bind _aiptr (`/Game/MyPlayer_BP.AIptr` _playerref))
  (if (`self.IsDay`)
    (set `self.IsDay` false)
    (set `self.MedicineTaken` (`/Game/AI/Sloth/Sloth_BP.MedicineTaken` (`/Game/AI/AI_BP.SlothRef` _aiptr)))
    (for (_array_element _array_index) (`/Game/MyPlayer_BP.myItems` _playerref)
      (`KismetArrayLibrary.Array_Set` (`self.ItemHidden`) _array_index (`/Game/Items/Item_BP.Hidden` _array_element)))
    (`/Game/UI/ItemBarUI.SaveItems` (`/Game/MyPlayer_BP.ItemBarW` _playerref))
    (`/Game/AI/AI_BP.SaveAIs` _aiptr)
    (`GameplayStatics.OpenLevel` "Night_Cycle")))

(event `Restart`
  (bind _aisdead (`self.AIsDead`))
  (bind _returnvalue (`|CreateWidget` "/Game/UI/ItemBarUI.ItemBarUI_C" (`GameplayStatics.GetPlayerController` 0)))
  (set `self.ItemBar` _returnvalue)
  (for (_ _array_index) _aisdead
    (`KismetArrayLibrary.Array_Set` _aisdead _array_index))
  (`GameplayStatics.OpenLevel` "Day_Cycle"))