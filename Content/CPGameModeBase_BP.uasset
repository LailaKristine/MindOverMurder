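; Game mode that runs a three-minute level timer and applies the saved sound mute options.
; BeginPlay sets base sound mixes from the GameInstance's SFX and music mute flags.
; Tick uses a one-second Delay to count up minutes and seconds, which GetSeconds returns as a total.
; At three minutes it calls the GameInstance's ChangeLevel, with a one-time Headmistress bedtime dialog if the player's HMRef is alive.
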(event `self.ReceiveBeginPlay`
  (`self.SetMuteForOption`))

(event `self.ReceiveTick`
  (params (DeltaSeconds :type "Float (single-precision)"))
  ;[1 1 1] Increment/Decrement Timer
  (`KismetSystemLibrary.Delay` 1.0)
  (if (== (`self.Minutes`) 3)
    (bind _asmy_player_bp (cast `/Game/MyPlayer_BP` (`GameplayStatics.GetPlayerPawn` 0)))
    (if (`/Game/AI/AI_BP.isAlive` (`/Game/AI/AI_BP.HMRef` (`/Game/MyPlayer_BP.AIptr` _asmy_player_bp)))
      (`/Engine/EditorBlueprintResources/StandardMacros.DoOnce` false
        (:`Completed`
          (bind _returnvalue (`|CreateWidget` "/Game/UI/Dialog.Dialog_C"))
          (`UserWidget.AddToViewport` _returnvalue 0)
          (set `/Game/UI/Dialog.TexArray` (`|MakeArray` (`|FormatText` "Headmistress: Time for bed!")) _returnvalue)
          (set `/Game/UI/Dialog.TextRow` 0 _returnvalue)
          (`KismetSystemLibrary.Delay` 5.0)
          (`Widget.RemoveFromParent` _returnvalue))))
    (bind _asgame_instance_bp (cast `/Game/GameInstance_BP` (`GameplayStatics.GetGameInstance`)))
    (`/Game/GameInstance_BP.ChangeLevel` _asgame_instance_bp)
    (elif (== (`self.Seconds`) 59)
      (set `self.Minutes` (+ (`self.Minutes`) 1))
      (set `self.Seconds` 0)
      (else
        (set `self.Seconds` (+ (`self.Seconds`) 1))))))

(fn `GetSeconds`
  (returns (NewParam :type Integer))
  (return (+ (* (`self.Minutes`) 60) (`self.Seconds`))))

(fn `SetMuteForOption`
  (bind _asgame_instance_bp (cast `/Game/GameInstance_BP` (`GameplayStatics.GetGameInstance`)))
  (`|ExecutionSequence`
    (:`then_0`
      (if (`/Game/GameInstance_BP.MuteSFXIsChecked` _asgame_instance_bp)
        (`GameplayStatics.SetBaseSoundMix` "/Game/Sound/MasterMuteSFXMix.MasterMuteSFXMix")
        (else
          (`GameplayStatics.SetBaseSoundMix` "/Game/Sound/MasterUnMuteSFXMix.MasterUnMuteSFXMix"))))
    (:`then_1`
      (if (`/Game/GameInstance_BP.MuteMusicIsChecked` _asgame_instance_bp)
        (`GameplayStatics.SetBaseSoundMix` "/Game/Sound/MasterMuteMusicMix.MasterMuteMusicMix")
        (else
          (`GameplayStatics.SetBaseSoundMix` "/Game/Sound/MasterUnMuteMusicMix.MasterUnMuteMusicMix"))))))

(fn `UserConstructionScript`)