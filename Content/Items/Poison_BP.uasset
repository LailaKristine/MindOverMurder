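; Poison_BP is a pickup item that the player can collect into the inventory, unless the janitor is in the room.
; Interact either shows a timed dialog and sets ActivatePlayerText on the player, or registers the poison with the player, adds it to the item bar and hides the actor.
; Drop unhides the same actor rather than spawning a new one.
; Use only prints a death message.
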(event `/Game/Items/Interact.Interact`
  ;[1 1 1] Pick up Poison: setting struct values and destroying actor
  (if (`/Game/AI/Janitor/Janitor_BP.IsInRoom` (`self.JanitorPtr`))
    (bind _returnvalue (`|CreateWidget` "/Game/UI/Dialog.Dialog_C"))
    (bind _output_get (set `self.DialogPtr` _returnvalue))
    (`UserWidget.AddToViewport` _output_get 0)
    (set `/Game/UI/Dialog.TexArray` (`self.DialogText`) (`self.DialogPtr`))
    (`KismetSystemLibrary.Delay` 3.0)
    (`Widget.RemoveFromParent` _output_get)
    (bind _asmy_player_bp (cast `/Game/MyPlayer_BP` (`GameplayStatics.GetPlayerPawn` 0)))
    (set `/Game/MyPlayer_BP.ActivatePlayerText` true _asmy_player_bp)
    (else
      (set `self.ItemStruct` (make `/Game/Items/ItemStruct` "/Game/Items/Icon/poison.poison" "Poison" true "Poison_BP_C"))
      (bind _asmy_player_bp_2 (cast `/Game/MyPlayer_BP` (`GameplayStatics.GetPlayerCharacter` 0)))
      (set `/Game/MyPlayer_BP.PoisonPtr` self _asmy_player_bp_2)
      (`/Game/UI/ItemBarUI.AddToInventory` (`/Game/MyPlayer_BP.ItemBarW` _asmy_player_bp_2) (`self.ItemStruct`))
      (`self.HideItem` true))))

(event `/Game/Items/Drop.Drop`
  ;[1 1 1] Drop
  (`self.HideItem` false))

(event `/Game/Items/Use.Use`
  ;[1 1 1] Use
  (`KismetSystemLibrary.PrintString` "You dead"))

(fn `UserConstructionScript`
  (`parent.UserConstructionScript`))