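; Medicine pickup item that the player can carry in the inventory and drop near a sloth.
; Interact fills the item struct, registers itself as the player's MedicinePtr, adds the entry to the item bar widget and hides the actor.
; Drop unhides the actor and, if its Box overlaps the referenced sloth, sets that sloth's MedicineText flag.
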(event `/Game/Items/Interact.Interact`
  ;[1 1 1] Pick up Medicine: setting struct values and destroying actor
  (set `self.ItemStruct` (make `/Game/Items/ItemStruct` "/Game/Items/Icon/Medicine-Icon.Medicine-Icon" "Medicine" true "Medicine_BP_C"))
  (bind _asmy_player_bp (cast `/Game/MyPlayer_BP` (`GameplayStatics.GetPlayerCharacter` 0)))
  (set `/Game/MyPlayer_BP.MedicinePtr` self _asmy_player_bp)
  (`/Game/UI/ItemBarUI.AddToInventory` (`/Game/MyPlayer_BP.ItemBarW` _asmy_player_bp) (`self.ItemStruct`))
  (`self.HideItem` true))

(event `/Game/Items/Drop.Drop`
  (bind _slothptr (`self.SlothPtr`))
  ;[1 1 1] Drop
  (`self.HideItem` false)
  (if (`PrimitiveComponent.IsOverlappingActor` (`self.Box`) _slothptr)
    (set `/Game/AI/Sloth/Sloth_BP.MedicineText` true _slothptr)))

(fn `UserConstructionScript`
  (`parent.UserConstructionScript`))