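; Lighter pickup item that the player can store in the inventory, drop and use.
; Interact builds its item struct, registers itself on MyPlayer_BP, adds the entry to the item bar and hides the actor; Drop unhides it.
; Use triggers KaplaRef's burn message when overlapping the player.
; Otherwise it uses HeaterRef if the player character overlaps the player pawn (itself), else prints a refusal.
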(event `/Game/Items/Interact.Interact`
  ;[1 1 1] Pick up Lighter: setting struct values and destroying actor
  (set `self.ItemStruct` (make `/Game/Items/ItemStruct` "/Game/Items/Icon/pngtree-vector-lighter-icon-png-image_4153864.pngtree-vector-lighter-icon-png-image_4153864" "Lighter" true "Lighter_BP_C"))
  (bind _asmy_player_bp (cast `/Game/MyPlayer_BP` (`GameplayStatics.GetPlayerCharacter` 0)))
  (set `/Game/MyPlayer_BP.LighterPtr` self _asmy_player_bp)
  (`/Game/UI/ItemBarUI.AddToInventory` (`/Game/MyPlayer_BP.ItemBarW` _asmy_player_bp) (`self.ItemStruct`))
  (`self.HideItem` true))

(event `/Game/Items/Drop.Drop`
  ;[1 1 1] Drop
  (`self.HideItem` false))

(event `/Game/Items/Use.Use`
  (bind _returnvalue (`GameplayStatics.GetPlayerPawn` 0))
  (bind _kaplaref (`self.KaplaRef`))
  (if (`self.IsOverlappingActor` _kaplaref _returnvalue)
    (message `/Game/Items/Burn.Burn` _kaplaref)
    (elif (`self.IsOverlappingActor` (`GameplayStatics.GetPlayerCharacter` 0) _returnvalue)
      (`/Game/Items/Use.Use` (`self.HeaterRef`))
      (else
        (`KismetSystemLibrary.PrintString` "You can't use that right now")))))

(fn `UserConstructionScript`
  (`parent.UserConstructionScript`))