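; WarningSign_BP is a warning sign item the player can pick up, drop and use.
; Interact fills an item struct, stores a self reference on MyPlayer_BP, adds the struct to the item bar inventory widget and hides the actor.
; Drop reveals the hidden actor again after a short delay, so it is never destroyed.
; Use only prints a death message.
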(event `/Game/Items/Interact.Interact`
  ;[1 1 1] Pick up Warning Sign: setting struct values and destroying actor
  (set `self.ItemStruct` (make `/Game/Items/ItemStruct` "/Game/Items/Icon/warningSign.warningSign" "Warning Sign" true "WarningSign_BP_C"))
  (bind _asmy_player_bp (cast `/Game/MyPlayer_BP` (`GameplayStatics.GetPlayerCharacter` 0)))
  (set `/Game/MyPlayer_BP.WarningSignPtr` self _asmy_player_bp)
  (`/Game/UI/ItemBarUI.AddToInventory` (`/Game/MyPlayer_BP.ItemBarW` _asmy_player_bp) (`self.ItemStruct`))
  (`self.HideItem` true))

(event `/Game/Items/Drop.Drop`
  ;[1 1 1] Drop
  (`KismetSystemLibrary.Delay` 1.5)
  (`self.HideItem` false))

(event `/Game/Items/Use.Use`
  ;[1 1 1] Use
  (`KismetSystemLibrary.PrintString` "You dead"))

(fn `UserConstructionScript`)