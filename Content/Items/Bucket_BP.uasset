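; Bucket item that the player can knock into a water spill, flagging the janitor that the player spilled it.
; Starts with its meshes hidden and the box, spill and bucket collision disabled.
; On Use while the player overlaps the box, it destroys the bucket, enables the visible spill and opens a Dialog widget.
; A DoOnce passes the dialog text and sets PlayerSpilled on the janitor reference.
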(event `self.ReceiveBeginPlay`
  (`parent.ReceiveBeginPlay`)
  (`SceneComponent.SetVisibility` (`self.StaticMesh`) false false)
  (`SceneComponent.SetVisibility` (`self.Bucket`) false false)
  (`PrimitiveComponent.SetCollisionEnabled` (`self.Box`) "NoCollision")
  (`PrimitiveComponent.SetCollisionEnabled` (`self.WaterSpill`) "NoCollision")
  (`PrimitiveComponent.SetCollisionEnabled` (`self.Bucket`) "NoCollision"))

(event `/Game/Items/Use.Use`
  (bind _waterspill (`self.WaterSpill`))
  (if (`PrimitiveComponent.IsOverlappingActor` (`self.Box`) (`self.PlayerRef`))
    (`ActorComponent.K2_DestroyComponent` (`self.Bucket`))
    (`SceneComponent.SetVisibility` _waterspill true false)
    (`PrimitiveComponent.SetCollisionEnabled` _waterspill "QueryAndPhysics")
    (bind _returnvalue (`|CreateWidget` "/Game/UI/Dialog.Dialog_C"))
    (bind _output_get (set `self.DialogRef` _returnvalue))
    (`UserWidget.AddToViewport` _output_get 0)
    (`/Engine/EditorBlueprintResources/StandardMacros.DoOnce` false
      (:`Completed`
        (set `/Game/UI/Dialog.TexArray` (`self.Dialog text`) (`self.DialogRef`))
        (set `/Game/AI/Janitor/Janitor_BP.PlayerSpilled` true (`self.JanitorRef`))))))

(fn `UserConstructionScript`
  (`parent.UserConstructionScript`))