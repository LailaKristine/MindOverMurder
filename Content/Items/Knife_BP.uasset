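; Knife item that the player can pick up, drop and use to attack, kept hidden for the first minute of play.
; Interact adds it to the inventory and registers it on the player, unless JanitorPtr.IsInRoom and IsInBasement are true and Hidden is false, which shows a brief dialog instead.
; Use spawns an Attack actor just ahead of the player, and Drop unhides the item.
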(event `self.ReceiveBeginPlay`
  (`parent.ReceiveBeginPlay`)
  (`self.HideItem` true)
  (`KismetSystemLibrary.Delay` 60.0)
  (`self.HideItem` false))

(event `/Game/Items/Interact.Interact`
  ;[1 1 1] Pick up Knife: setting struct values and calling disable function from parent
  (if (`/Game/AI/Janitor/Janitor_BP.IsInRoom` (`self.JanitorPtr`))
    (if (`self.IsInBasement`)
      (if (`self.Hidden`)
        (set `self.ItemStruct` (make `/Game/Items/ItemStruct` "/Game/Items/Icon/knife.knife" "Knife" true "Knife_BP_C") :!label _label)
        (bind _asmy_player_bp (cast `/Game/MyPlayer_BP` (`GameplayStatics.GetPlayerCharacter` 0)))
        (set `/Game/MyPlayer_BP.KnifePtr` self _asmy_player_bp)
        (`/Game/UI/ItemBarUI.AddToInventory` (`/Game/MyPlayer_BP.ItemBarW` _asmy_player_bp) (`self.ItemStruct`))
        (`self.HideItem` true)
        (set `/Game/MyPlayer_BP.KnifePickedUp` true _asmy_player_bp)
        (else
          (bind _returnvalue (`|CreateWidget` "/Game/UI/Dialog.Dialog_C"))
          (bind _output_get (set `self.DialogPtr` _returnvalue))
          (`UserWidget.AddToViewport` _output_get 0)
          (set `/Game/UI/Dialog.TexArray` (`self.DialogText`) (`self.DialogPtr`))
          (`KismetSystemLibrary.Delay` 3.0)
          (`Widget.RemoveFromParent` _output_get)
          (bind _asmy_player_bp_2 (cast `/Game/MyPlayer_BP` (`GameplayStatics.GetPlayerPawn` 0)))
          (set `/Game/MyPlayer_BP.ActivatePlayerText` true _asmy_player_bp_2)))
      (else
        (goto _label)))
    (else
      (goto _label))))

(event `/Game/Items/Drop.Drop`
  ;[1 1 1] Pick up Knife: setting struct values and calling disable function from parent
  (`self.HideItem` false))

(event `/Game/Items/Use.Use`
  (bind _returnvalue (`GameplayStatics.GetPlayerPawn` 0))
  ;[1 1 1] Use
  (`|SpawnActorFromClass` "/Game/Items/Attack.Attack_C" (`KismetMathLibrary.Conv_VectorToTransform` (+ (`SceneComponent.K2_GetComponentLocation` (`Actor.RootComponent` _returnvalue)) (* (`self.GetActorForwardVector` _returnvalue) 20))) "Undefined" "OverrideRootScale" null null))

(event `self.ReceiveActorBeginOverlap`
  (params (OtherActor :type "Actor Object Reference"))
  (`parent.ReceiveActorBeginOverlap` OtherActor))

(fn `UserConstructionScript`
  (`parent.UserConstructionScript`))