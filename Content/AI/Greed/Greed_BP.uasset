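; Greed NPC character that talks to the player, can die by burning and can appear as a ghost at night.
; Use shows camera-facing text chosen by Kapla build state while in the room with Sloth alive, zeroing speed briefly, though Tick resets it.
; BeginPlay reads the game instance to toggle cold breath and apply ghost materials.
; A splatter emitter spawns at Sloth's stab point, with a collision handler for randomized blood decals.
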(event `/Game/Items/Use.Use`
  (bind _textrender (`self.TextRender`))
  (bind _charactermovement (`self.CharacterMovement`))
  ;[1 1 1] Use/Activate Text Dialog
  (if (`self.IsInRoom`)
    (if (`/Game/AI/AI_BP.isAlive` (`self.SlothRef`))
      (if (`/Game/Assets/Kapla_BP.IsBuilt` (`self.KaplaRef`))
        (`TextRenderComponent.K2_SetText` _textrender (`|GetArrayItem` (`self.NpcText`) 1))
        (else
          (`TextRenderComponent.K2_SetText` _textrender (`|GetArrayItem` (`self.NpcText`)))))
      (`SceneComponent.K2_SetWorldRotation` _textrender (.rotation (`self.GetTransform` (`self.CameraRef`))) false false)
      (`SceneComponent.K2_AddLocalRotation` _textrender (struct :`Yaw` -180.0) false false)
      (set `CharacterMovementComponent.MaxWalkSpeed` 0.0 _charactermovement)
      (`SceneComponent.SetVisibility` (`self.TextRender`) true false)
      (`KismetSystemLibrary.Delay` 5.0)
      (`SceneComponent.SetVisibility` (`self.TextRender`) false false)
      (set `CharacterMovementComponent.MaxWalkSpeed` 150.0 _charactermovement))))

(event `/Game/Items/Burn.Burn`
  (`self.Death`))

(event `self.ReceiveTick`
  (params (DeltaSeconds :type "Float (single-precision)"))
  (`self.Walk`))

(event `Walk`
  ;[1 1 1] Walk/Run Speed
  (set `CharacterMovementComponent.MaxWalkSpeed` 200.0 (`self.CharacterMovement`)))

(event `Run`
  ;[1 1 1] Walk/Run Speed
  (set `CharacterMovementComponent.MaxWalkSpeed` 400.0 (`self.CharacterMovement`)))

(event `self.ReceiveBeginPlay`
  (bind _coldbreath (`self.ColdBreath`))
  (bind _asgame_instance_bp (cast `/Game/GameInstance_BP` (`GameplayStatics.GetGameInstance`)))
  (if (`/Game/GameInstance_BP.IsDay` _asgame_instance_bp)
    (`SceneComponent.SetVisibility` _coldbreath false false)
    (else
      (`SceneComponent.SetVisibility` _coldbreath true false)
      (if (`|GetArrayItem` (`/Game/GameInstance_BP.AIsDead` _asgame_instance_bp))
        (`self.Ghostify`)))))

(event `SpawnSplatter`
  ;[1 1 1] Spawn BloodParticle - KillSloth
  (bind _returnvalue (`GameplayStatics.SpawnEmitterAtLocation` "/Game/Assets/Particles/Splatter_PS.Splatter_PS" (`SceneComponent.K2_GetComponentLocation` (`/Game/AI/Sloth/Sloth_BP.StabRef` (`self.SlothRef`)))))
  (remove `ParticleSystemComponent.OnParticleCollide` _returnvalue (delegate `On Particle Collide`)))

(event `On Particle Collide`
  (params (EventName :type Name) (EmitterTime :type "Float (double-precision)") (ParticleTime :type Integer) (Location :type "Vector Structure") (Velocity :type "Vector Structure") (Direction :type "Vector Structure") (Normal :type "Vector Structure") (BoneName :type Name) (PhysMat :type "PhysicalMaterial Object Reference"))
  ;[1 1 1] Spawn BloodParticle - KillSloth
  (bind _returnvalue (`KismetMaterialLibrary.CreateDynamicMaterialInstance` "/Game/Assets/Particles/Splatter_Decal_M.Splatter_Decal_M"))
  (`MaterialInstanceDynamic.SetScalarParameterValue` _returnvalue "None" (`KismetMathLibrary.Conv_IntToDouble` (`KismetMathLibrary.RandomInteger` 11)))
  (`GameplayStatics.SpawnDecalAtLocation` _returnvalue (`KismetMathLibrary.Conv_DoubleToVector` (`KismetMathLibrary.RandomFloatInRange` 20.0 50.0)) Location (`KismetMathLibrary.Conv_VectorToRotator` Normal) 20.0))

(fn `Ghostify`
  (bind _mesh (`self.Mesh`))
  (set `self.IsGhost` true)
  (`PrimitiveComponent.SetMaterial` _mesh 1 "/Game/Assets/Materials/ShirtMC_Ghost_M1.ShirtMC_Ghost_M1")
  (`PrimitiveComponent.SetMaterial` _mesh 2 "/Game/Assets/Materials/DressMC_Ghost_M.DressMC_Ghost_M")
  (`PrimitiveComponent.SetMaterial` _mesh 3 "/Game/Assets/Materials/SkinMC_Ghost_M.SkinMC_Ghost_M")
  (`PrimitiveComponent.SetMaterial` _mesh 4 "/Game/Assets/Materials/PantsGreed_Ghost_M.PantsGreed_Ghost_M")
  (`PrimitiveComponent.SetMaterial` _mesh 5 "/Game/Assets/Materials/HairGreed_Ghost_M.HairGreed_Ghost_M"))

(fn `UserConstructionScript`)