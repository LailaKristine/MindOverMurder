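; GreedController_BP is the AI controller for the Greed character, running the Greed_BT behavior tree on its pawn.
; On BeginPlay it caches the Greed pawn and seeds the blackboard with door, patrol direction and wait time values.
; Every tick it copies pawn state flags and the game instance's day flag into the blackboard.
; Walk, Run and SpawnSplatter events forward directly to the pawn.
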(event `self.ReceiveTick`
  (params (DeltaSeconds :type "Float (single-precision)"))
  (`BlackboardComponent.SetValueAsBool` (`AIBlueprintHelperLibrary.GetBlackboard` null) "Start task one" (`/Game/AI/Greed/Greed_BP.DoTask1` (`self.MyPawn`)))
  (`BlackboardComponent.SetValueAsBool` (`AIBlueprintHelperLibrary.GetBlackboard` null) "WalkPatrol" (`/Game/AI/Greed/Greed_BP.WalkPatrol` (`self.MyPawn`)))
  (`BlackboardComponent.SetValueAsBool` (`AIBlueprintHelperLibrary.GetBlackboard` null) "HoldingMedicine" (`/Game/AI/Greed/Greed_BP.HoldingMedicine` (`self.MyPawn`)))
  (`BlackboardComponent.SetValueAsBool` (`AIBlueprintHelperLibrary.GetBlackboard` null) "Alive?" (`/Game/AI/AI_BP.isAlive` (`self.MyPawn`)))
  (bind _asgame_instance_bp (cast `/Game/GameInstance_BP` (`GameplayStatics.GetGameInstance`)))
  (`BlackboardComponent.SetValueAsBool` (`AIBlueprintHelperLibrary.GetBlackboard` null) "isDay" (`/Game/GameInstance_BP.IsDay` _asgame_instance_bp)))

(event `self.ReceiveBeginPlay`
  (bind _returnvalue (`AIBlueprintHelperLibrary.GetBlackboard` null))
  (`self.RunBehaviorTree` "/Game/AI/Greed/Greed_BT.Greed_BT")
  (bind _asgreed_bp (cast `/Game/AI/Greed/Greed_BP` (`self.K2_GetPawn`)))
  (bind _output_get (set `self.MyPawn` _asgreed_bp))
  (`BlackboardComponent.SetValueAsBool` (`AIBlueprintHelperLibrary.GetBlackboard` null) "DoorFound" (`/Game/AI/Greed/Greed_BP.DoorDone` _output_get))
  (`BlackboardComponent.SetValueAsInt` _returnvalue "Direction" 1)
  (`BlackboardComponent.SetValueAsFloat` _returnvalue "WaitTime" (`/Game/AI/PatrolPath.WaitTime` (`/Game/AI/Greed/Greed_BP.PatrolPath` (`self.MyPawn`)))))

(event `Walk`
  (`/Game/AI/Greed/Greed_BP.Walk` (stale `self.ReceiveBeginPlay` _output_get)))

(event `Run`
  (`/Game/AI/Greed/Greed_BP.Run` (stale `self.ReceiveBeginPlay` _output_get)))

(event `SpawnSplatter`
  (`/Game/AI/Greed/Greed_BP.SpawnSplatter` (stale `self.ReceiveBeginPlay` _output_get)))

(fn `UserConstructionScript`)