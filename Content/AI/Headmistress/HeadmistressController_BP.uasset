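; AI controller for the Headmistress NPC that runs her behavior tree and feeds it game state.
; BeginPlay seeds the blackboard with door, patrol direction and wait time values from the pawn.
; Tick copies alive, day, sloth-waking and player door-transit flags from the pawn, game instance and player reference every frame.
; AI perception updates whether she can see the player, and Walk and Run events forward to the pawn.
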(event `self.ReceiveBeginPlay`
  (bind _returnvalue (`AIBlueprintHelperLibrary.GetBlackboard` null))
  (`self.RunBehaviorTree` "/Game/AI/Headmistress/Headmistress_BT.Headmistress_BT")
  (bind _asheadmistress_bp (cast `/Game/AI/Headmistress/Headmistress_BP` (`self.K2_GetPawn`)))
  (bind _output_get (set `self.MyPawn` _asheadmistress_bp))
  (`BlackboardComponent.SetValueAsBool` (`AIBlueprintHelperLibrary.GetBlackboard` null) "DoorFound" (`/Game/AI/Headmistress/Headmistress_BP.DoorDone` _output_get))
  (`BlackboardComponent.SetValueAsInt` _returnvalue "Direction" 1)
  (`BlackboardComponent.SetValueAsFloat` _returnvalue "WaitTime" (`/Game/AI/PatrolPath.WaitTime` (`/Game/AI/Headmistress/Headmistress_BP.PatrolPathTask1` (`self.MyPawn`)))))

(event `self.ReceiveTick`
  (params (DeltaSeconds :type "Float (single-precision)"))
  (`BlackboardComponent.SetValueAsBool` (`AIBlueprintHelperLibrary.GetBlackboard` null) "Alive?" (`/Game/AI/AI_BP.isAlive` (`self.MyPawn`)))
  (bind _asgame_instance_bp (cast `/Game/GameInstance_BP` (`GameplayStatics.GetGameInstance`)))
  (`BlackboardComponent.SetValueAsBool` (`AIBlueprintHelperLibrary.GetBlackboard` null) "isDay" (`/Game/GameInstance_BP.IsDay` _asgame_instance_bp))
  (`BlackboardComponent.SetValueAsBool` (`AIBlueprintHelperLibrary.GetBlackboard` null) "WakeSloth" (`/Game/AI/Headmistress/Headmistress_BP.WakeSloth` (`self.MyPawn`)))
  (`BlackboardComponent.SetValueAsBool` (`AIBlueprintHelperLibrary.GetBlackboard` null) "PlayerGoThroughDoor" (`/Game/MyPlayer_BP.GoingThroughDoor` (`/Game/AI/Headmistress/Headmistress_BP.PlayerRef` (`self.MyPawn`)))))

(event `Walk`
  (`/Game/AI/Headmistress/Headmistress_BP.Walk` (stale `self.ReceiveBeginPlay` _output_get)))

(event `Run`
  (`/Game/AI/Headmistress/Headmistress_BP.Run` (stale `self.ReceiveBeginPlay` _output_get)))

(event `self.AIPerception.OnTargetPerceptionUpdated`
  (params (Actor :type "Actor Object Reference") (Stimulus :type "AIStimulus Structure"))
  (cast `/Game/MyPlayer_BP` Actor)
  (`BlackboardComponent.SetValueAsBool` (`AIBlueprintHelperLibrary.GetBlackboard` null) "CanSeePlayer" (`.bSuccessfullySensed` (break `AIStimulus` Stimulus))))

(fn `UserConstructionScript`)