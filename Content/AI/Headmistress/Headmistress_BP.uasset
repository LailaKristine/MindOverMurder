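; Headmistress_BP is the Blueprint for the Headmistress AI character, setting her movement speed and cold-breath effect.
; On BeginPlay she starts at walking speed, and the ColdBreath component is hidden during the day and shown otherwise, based on IsDay in GameInstance_BP.
; Walk and Run events switch CharacterMovement between a slower and a faster max speed.
; An unconnected fragment would destroy a component once HeaterRef is fixed, but never runs.
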(event `self.ReceiveBeginPlay`
  (`self.Walk`)
  (bind _asgame_instance_bp (cast `/Game/GameInstance_BP` (`GameplayStatics.GetGameInstance`)))
  (if (`/Game/GameInstance_BP.IsDay` _asgame_instance_bp)
    (`SceneComponent.SetVisibility` (`self.ColdBreath`) false false)
    (else
      (`SceneComponent.SetVisibility` (`self.ColdBreath`) true false))))

(event `Walk`
  (set `CharacterMovementComponent.MaxWalkSpeed` 150.0 (`self.CharacterMovement`)))

(event `Run`
  (set `CharacterMovementComponent.MaxWalkSpeed` 300.0 (`self.CharacterMovement`)))

(event `self.ReceiveTick`
  (params (DeltaSeconds :type "Float (single-precision)")))

(fn `UserConstructionScript`)