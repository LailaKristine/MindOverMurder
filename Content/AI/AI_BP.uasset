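; AI_BP is an AI actor Blueprint that tracks alive or dead state for four characters: Greed, HM, Janitor and Sloth.
; BeginPlay gathers their references into an array and clears IsAlive on those flagged in the game instance's AIsDead array.
; Death tips the actor over and clears IsAlive.
; SaveAIs inserts true into AIsDead at each dead character's index, shifting later entries rather than overwriting them.
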(event `self.ReceiveBeginPlay`
  (set `self.AllChildren` (`|MakeArray` (`self.GreedRef`) (`self.HMRef`) (`self.JanitorRef`) (`self.SlothRef`) :!type "/Game/AI/AI_BP Object Reference"))
  (bind _asgame_instance_bp (cast `/Game/GameInstance_BP` (`GameplayStatics.GetGameInstance`)))
  (for (_array_element _array_index) (`/Game/GameInstance_BP.AIsDead` _asgame_instance_bp)
    (if _array_element
      (set `/Game/AI/AI_BP.isAlive` false (`|GetArrayItem` (`self.AllChildren`) _array_index)))))

(fn `Death`
  (`self.K2_SetActorRotation` (`KismetMathLibrary.MakeRotator` -90.0))
  (set `self.isAlive` false)
  (`KismetSystemLibrary.PrintString` (`KismetStringLibrary.Conv_ObjectToString` self)))

(fn `SaveAIs`
  (for (_array_element _array_index) (`self.AllChildren`)
    (if (not (`/Game/AI/AI_BP.isAlive` _array_element))
      (bind _asgame_instance_bp (cast `/Game/GameInstance_BP` (`GameplayStatics.GetGameInstance`)))
      (`KismetArrayLibrary.Array_Insert` (`/Game/GameInstance_BP.AIsDead` _asgame_instance_bp) true _array_index))))

(fn `UserConstructionScript`)