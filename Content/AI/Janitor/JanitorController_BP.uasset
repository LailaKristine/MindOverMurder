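; AI controller for the Janitor NPC that runs its behavior tree and feeds it state from the pawn and game.
; On BeginPlay it starts Janitor_BT, caches the Janitor pawn and seeds blackboard keys for door progress, patrol direction and wait time.
; Every tick it copies the pawn's spill and alive flags and the game instance's day state into the blackboard.
; Walk and Run events forward to the pawn.
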(event `self.ReceiveTick`
  (params (DeltaSeconds :type "Float (single-precision)"))
  (`BlackboardComponent.SetValueAsBool` (`AIBlueprintHelperLibrary.GetBlackboard` null) "PlayerSpilled" (`/Game/AI/Janitor/Janitor_BP.PlayerSpilled` (`self.MyPawn`)))
  (`BlackboardComponent.SetValueAsBool` (`AIBlueprintHelperLibrary.GetBlackboard` null) "Alive?" (`/Game/AI/AI_BP.isAlive` (`self.MyPawn`)))
  (bind _asgame_instance_bp (cast `/Game/GameInstance_BP` (`GameplayStatics.GetGameInstance`)))
  (`BlackboardComponent.SetValueAsBool` (`AIBlueprintHelperLibrary.GetBlackboard` null) "isDay" (`/Game/GameInstance_BP.IsDay` _asgame_instance_bp)))

(event `self.ReceiveBeginPlay`
  (bind _returnvalue (`AIBlueprintHelperLibrary.GetBlackboard` null))
  (`self.RunBehaviorTree` "/Game/AI/Janitor/Janitor_BT.Janitor_BT")
  (bind _asjanitor_bp (cast `/Game/AI/Janitor/Janitor_BP` (`self.K2_GetPawn`)))
  (bind _output_get (set `self.MyPawn` _asjanitor_bp))
  (`BlackboardComponent.SetValueAsBool` (`AIBlueprintHelperLibrary.GetBlackboard` null) "DoorFound" (`/Game/AI/Janitor/Janitor_BP.DoorDone` _output_get))
  (`BlackboardComponent.SetValueAsInt` _returnvalue "Direction" 1)
  (`BlackboardComponent.SetValueAsFloat` _returnvalue "WaitTime" (`/Game/AI/PatrolPath.WaitTime` (`/Game/AI/Janitor/Janitor_BP.PatrolPathWork` (`self.MyPawn`)))))

(event `Walk`
  (`/Game/AI/Janitor/Janitor_BP.Walk` (stale `self.ReceiveBeginPlay` _output_get)))

(event `Run`
  (`/Game/AI/Janitor/Janitor_BP.Run` (stale `self.ReceiveBeginPlay` _output_get)))

(fn `UserConstructionScript`)