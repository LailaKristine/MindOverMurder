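; Janitor_BP is the janitor AI character, with movement speed switching and a cold breath effect tied to time of day.
; Walk and Run events set CharacterMovement max speed, and the janitor starts at walking speed.
; After a short startup delay, it reads IsDay from GameInstance_BP once and shows ColdBreath only when it is not day.
; A heater-fixed check that would destroy a component is left unconnected and never runs.
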(event `self.ReceiveBeginPlay`
  (bind _coldbreath (`self.ColdBreath`))
  (`self.Walk`)
  (`KismetSystemLibrary.Delay` 2.0)
  (bind _asgame_instance_bp (cast `/Game/GameInstance_BP` (`GameplayStatics.GetGameInstance`)))
  (if (`/Game/GameInstance_BP.IsDay` _asgame_instance_bp)
    (`SceneComponent.SetVisibility` _coldbreath false false)
    (else
      (`SceneComponent.SetVisibility` _coldbreath true false))))

(event `Walk`
  (set `CharacterMovementComponent.MaxWalkSpeed` 150.0 (`self.CharacterMovement`)))

(event `Run`
  (set `CharacterMovementComponent.MaxWalkSpeed` 400.0 (`self.CharacterMovement`)))

(event `self.ReceiveTick`
  (params (DeltaSeconds :type "Float (single-precision)")))

(fn `UserConstructionScript`)