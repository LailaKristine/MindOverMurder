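; AI controller for the Sloth enemy or NPC that runs its behavior tree and keeps the blackboard in sync with the game.
; On BeginPlay it starts Sloth_BT, caches the possessed Sloth pawn and seeds door, patrol direction and wait time keys.
; Every tick it copies pawn state and GameInstance day and medicine flags into the blackboard.
; Walk and Run events forward to the pawn.
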(event `self.ReceiveBeginPlay`
  (bind _returnvalue (`AIBlueprintHelperLibrary.GetBlackboard` null))
  (`self.RunBehaviorTree` "/Game/AI/Sloth/Sloth_BT.Sloth_BT")
  (bind _assloth_bp (cast `/Game/AI/Sloth/Sloth_BP` (`self.K2_GetPawn`)))
  (bind _output_get (set `self.MyPawn` _assloth_bp))
  (`BlackboardComponent.SetValueAsBool` (`AIBlueprintHelperLibrary.GetBlackboard` null) "DoorFound" (`/Game/AI/Sloth/Sloth_BP.DoorDone` _output_get))
  (`BlackboardComponent.SetValueAsInt` _returnvalue "Direction" 1)
  (`BlackboardComponent.SetValueAsFloat` _returnvalue "WaitTime" (`/Game/AI/PatrolPath.WaitTime` (`/Game/AI/Sloth/Sloth_BP.PatrolPath` (`self.MyPawn`)))))

(event `self.ReceiveTick`
  (params (DeltaSeconds :type "Float (single-precision)"))
  (`BlackboardComponent.SetValueAsBool` (`AIBlueprintHelperLibrary.GetBlackboard` null) "isAwake" (`/Game/AI/Sloth/Sloth_BP.Awake?` (`self.MyPawn`)))
  (`BlackboardComponent.SetValueAsBool` (`AIBlueprintHelperLibrary.GetBlackboard` null) "Alive?" (`/Game/AI/AI_BP.isAlive` (`self.MyPawn`)))
  (bind _asgame_instance_bp (cast `/Game/GameInstance_BP` (`GameplayStatics.GetGameInstance`)))
  (`BlackboardComponent.SetValueAsBool` (`AIBlueprintHelperLibrary.GetBlackboard` null) "isDay" (`/Game/GameInstance_BP.IsDay` _asgame_instance_bp))
  (`BlackboardComponent.SetValueAsBool` (`AIBlueprintHelperLibrary.GetBlackboard` null) "MedicineTaken" (`/Game/GameInstance_BP.MedicineTaken` _asgame_instance_bp))
  (`BlackboardComponent.SetValueAsBool` (`AIBlueprintHelperLibrary.GetBlackboard` null) "PlayerIsInRoom" (`/Game/AI/Sloth/Sloth_BP.PlayerIsInRoom` (`self.MyPawn`)))
  (`BlackboardComponent.SetValueAsBool` (`AIBlueprintHelperLibrary.GetBlackboard` null) "AllowPatrol" (`/Game/AI/Sloth/Sloth_BP.AllowPatrol` (`self.MyPawn`))))

(event `Walk`
  (`/Game/AI/Sloth/Sloth_BP.Walk` (stale `self.ReceiveBeginPlay` _output_get)))

(event `Run`
  (`/Game/AI/Sloth/Sloth_BP.Run` (stale `self.ReceiveBeginPlay` _output_get)))

(fn `UserConstructionScript`)