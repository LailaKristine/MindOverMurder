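; WaterSpill_BP is a water spill hazard that starts hidden, with its hazard box's collision disabled.
; When the janitor enters the trigger Box1, a short delay reveals the mesh, enables the hazard box and marks the water spilled.
; The hazard box kills the headmistress or player once each, while overlapping the warning sign destroys the spill and sets the player's HMSaved flag.
; Box1 also toggles the player's text visibility flag around an active spill.
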(event `self.ReceiveBeginPlay`
  (`PrimitiveComponent.SetCollisionEnabled` (`self.Box`) "NoCollision")
  (`SceneComponent.SetVisibility` (`self.StaticMesh`) false false))

(event `self.Box.OnComponentBeginOverlap`
  (params (OverlappedComponent :type "PrimitiveComponent Object Reference") (OtherActor :type "Actor Object Reference") (OtherComp :type "PrimitiveComponent Object Reference") (OtherBodyIndex :type Integer) (bFromSweep :type Boolean) (SweepResult :type "HitResult Structure (by ref)"))
  (bind _headmistressref (`self.HeadmistressRef`))
  (bind _playerref (`self.PlayerRef`))
  (if (== OtherActor _headmistressref)
    (`/Engine/EditorBlueprintResources/StandardMacros.DoOnce` false
      (:`Completed`
        (`/Game/AI/AI_BP.Death` _headmistressref)))
    (elif (== OtherActor (`self.WarningSignRef`))
      (`self.K2_DestroyActor`)
      (set `/Game/MyPlayer_BP.HMSaved` true (`self.PlayerRef`))
      (elif (== OtherActor _playerref)
        (`/Engine/EditorBlueprintResources/StandardMacros.DoOnce` false
          (:`Completed`
            (`/Game/MyPlayer_BP.Death` _playerref 0)))))))

(event `self.Box1.OnComponentEndOverlap`
  (params (OverlappedComponent :type "PrimitiveComponent Object Reference") (OtherActor :type "Actor Object Reference") (OtherComp :type "PrimitiveComponent Object Reference") (OtherBodyIndex :type Integer))
  (bind _asmy_player_bp (cast `/Game/MyPlayer_BP` OtherActor))
  (set `/Game/MyPlayer_BP.SetTextVisibility` false _asmy_player_bp))

(event `self.Box1.OnComponentBeginOverlap`
  (params (OverlappedComponent :type "PrimitiveComponent Object Reference") (OtherActor :type "Actor Object Reference") (OtherComp :type "PrimitiveComponent Object Reference") (OtherBodyIndex :type Integer) (bFromSweep :type Boolean) (SweepResult :type "HitResult Structure (by ref)"))
  (if (== (`self.JanitorRef`) OtherActor)
    (`KismetSystemLibrary.Delay` 1.0)
    (`PrimitiveComponent.SetCollisionEnabled` (`self.Box`) "QueryAndPhysics")
    (`SceneComponent.SetVisibility` (`self.StaticMesh`) true false)
    (set `self.waterSpilled` true)
    (elif (`self.waterSpilled`)
      (bind _asmy_player_bp (cast `/Game/MyPlayer_BP` OtherActor))
      (set `/Game/MyPlayer_BP.SetTextVisibility` true _asmy_player_bp))))

(fn `UserConstructionScript`)