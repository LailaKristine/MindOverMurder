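; Closet actor with two swinging doors that open and close on use or when a specific actor, GreedRef, passes its trigger box.
; The Use event flip-flops a timeline forward and in reverse to drive the relative yaw of both doors.
; A separate timeline opens the doors when GreedRef enters BoxAI, then reverses on exit as the box destroys itself, making that trigger one-shot.
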(event `/Game/Items/Use.Use`
  (`/Engine/EditorBlueprintResources/StandardMacros.FlipFlop`
    (:`A`
      (bind (_direction _ldoor _rdoor) (`Timeline|DoorTimeLineRotation` :!label _label)
        (:`Update`
          (`SceneComponent.K2_SetRelativeRotation` (`self.LDoor`) (`KismetMathLibrary.MakeRotator` 0.0 0.0 _ldoor) false false)
          (`SceneComponent.K2_SetRelativeRotation` (`self.RDoor`) (`KismetMathLibrary.MakeRotator` 0.0 0.0 _rdoor) false false))))
    (:`B`
      (goto _label :!via `Reverse`))))

(event `self.BoxAI.OnComponentBeginOverlap`
  (params (OverlappedComponent :type "PrimitiveComponent Object Reference") (OtherActor :type "Actor Object Reference") (OtherComp :type "PrimitiveComponent Object Reference") (OtherBodyIndex :type Integer) (bFromSweep :type Boolean) (SweepResult :type "HitResult Structure (by ref)"))
  (if (== OtherActor (`self.GreedRef`))
    (bind (_direction _ldoor _rdoor) (`Timeline|Timeline_0` :!label _label_2)
      (:`Update`
        (`SceneComponent.K2_SetRelativeRotation` (`self.LDoor`) (`KismetMathLibrary.MakeRotator` 0.0 0.0 _ldoor) false false)
        (`SceneComponent.K2_SetRelativeRotation` (`self.RDoor`) (`KismetMathLibrary.MakeRotator` 0.0 0.0 _rdoor) false false)))))

(event `self.BoxAI.OnComponentEndOverlap`
  (params (OverlappedComponent :type "PrimitiveComponent Object Reference") (OtherActor :type "Actor Object Reference") (OtherComp :type "PrimitiveComponent Object Reference") (OtherBodyIndex :type Integer))
  (if (== OtherActor (`self.GreedRef`))
    (`|ExecutionSequence`
      (:`then_0`
        (goto _label_2 :!via `Reverse`))
      (:`then_1`
        (`ActorComponent.K2_DestroyComponent` (`self.BoxAI`))))))

(fn `UserConstructionScript`)