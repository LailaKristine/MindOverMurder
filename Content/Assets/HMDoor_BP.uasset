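; A door actor that swings open when the player enters its box and then kills the player after a monster sound.
; The overlap plays a timeline that drives the door's yaw.
; Tick polls that yaw for exact quarter-turn and half-turn values, turning door collision off or on respectively.
; Either match feeds a shared DoOnce that plays the sound, waits briefly, then calls Death on MyPlayer_BP.
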(event `self.ReceiveTick`
  (params (DeltaSeconds :type "Float (single-precision)"))
  (if (== (stale `self.Box.OnComponentBeginOverlap` _doorrotationz) 180.0)
    (`PrimitiveComponent.SetCollisionEnabled` (`self.Door`) "QueryAndPhysics")
    (bind _asmy_player_bp (cast `/Game/MyPlayer_BP` (`GameplayStatics.GetPlayerPawn` 0) :!label _label))
    (`/Engine/EditorBlueprintResources/StandardMacros.DoOnce` false
      (:`Completed`
        (`GameplayStatics.PlaySoundAtLocation` "/Game/Sound/Monster_jafs.Monster_jafs" (`self.K2_GetActorLocation` self) (struct) 1.0 1.0 0.0 null null null)
        (`KismetSystemLibrary.Delay` 2.5)
        (`/Game/MyPlayer_BP.Death` _asmy_player_bp 3)))
    (elif (== (stale `self.Box.OnComponentBeginOverlap` _doorrotationz) 90.0)
      (`PrimitiveComponent.SetCollisionEnabled` (`self.Door`) "NoCollision")
      (goto _label))))

(event `self.Box.OnComponentBeginOverlap`
  (params (OverlappedComponent :type "PrimitiveComponent Object Reference") (OtherActor :type "Actor Object Reference") (OtherComp :type "PrimitiveComponent Object Reference") (OtherBodyIndex :type Integer) (bFromSweep :type Boolean) (SweepResult :type "HitResult Structure (by ref)"))
  (if (== OtherActor (`GameplayStatics.GetPlayerPawn` 0))
    (bind (_direction _doorrotationz) (`Timeline|DoorTimeLine`)
      (:`Update`
        (`SceneComponent.K2_SetRelativeRotation` (`self.Door`) (`KismetMathLibrary.MakeRotator` 0.0 0.0 _doorrotationz) false false)))))

(fn `UserConstructionScript`)