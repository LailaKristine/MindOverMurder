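; Kapla block tower actor that can be knocked down into a pile or set on fire.
; BeginPlay caches three build-stage components, hides them and disables their collision along with the pile's.
; Use hides the tower, shows the pile with physics-only collision and flags it Fallen.
; Burn does the same swap, but reveals fire particles, flags it Burned and sends BurnMessage to the first overlapping Greed_BP.
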(event `self.ReceiveBeginPlay`
  (bind _array (`|MakeArray` (`self.build_1`) (`self.build_2`) (`self.build_3`)))
  (set `self.Tower` _array)
  (for _array_element _array
    (`SceneComponent.SetVisibility` _array_element false false)
    (`PrimitiveComponent.SetCollisionEnabled` _array_element "NoCollision")
    (`PrimitiveComponent.SetCollisionEnabled` (`self.pile`) "NoCollision")))

(event `/Game/Items/Use.Use`
  (bind _pile (`self.pile`))
  (for _array_element (`self.Tower`)
    (`SceneComponent.SetVisibility` _array_element false false)
    (`PrimitiveComponent.SetCollisionEnabled` _array_element "PhysicsOnly"))
  (`SceneComponent.SetVisibility` _pile true false)
  (`PrimitiveComponent.SetCollisionEnabled` _pile "PhysicsOnly")
  (set `self.Fallen` true))

(event `/Game/Items/Burn.Burn`
  (bind _pile (`self.pile`))
  (`SceneComponent.SetVisibility` (`self.ParticleSystemFire`) true false)
  (for _array_element (`self.Tower`)
    (`SceneComponent.SetVisibility` _array_element false false)
    (`PrimitiveComponent.SetCollisionEnabled` _array_element "PhysicsOnly"))
  (`SceneComponent.SetVisibility` _pile true false)
  (`PrimitiveComponent.SetCollisionEnabled` _pile "PhysicsOnly")
  (set `self.Burned` true)
  (for _array_element_2 (`self.GetOverlappingActors` "/Game/AI/Greed/Greed_BP.Greed_BP_C")
    (message `/Game/Items/Burn.Burn` _array_element_2)
    (break)))

(fn `UserConstructionScript`)