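; Locked door actor that responds to a Use event with a locked sound and a dialog message.
; Use plays the sound at the door's location, adds a new Dialog widget to the viewport and passes it the DoorText content.
; A DoOnce gate blocks repeat uses until ResetDialog reopens it after a short delay.
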(event `/Game/Items/Use.Use`
  (`/Engine/EditorBlueprintResources/StandardMacros.DoOnce` false :!label _label
    (:`Completed`
      (`GameplayStatics.PlaySoundAtLocation` "/Game/Sound/LockedDoor.LockedDoor" (`self.K2_GetActorLocation` self) (struct) 1.0 1.0 0.0 null null null)
      (bind _returnvalue (`|CreateWidget` "/Game/UI/Dialog.Dialog_C"))
      (bind _output_get (set `self.DialogUIRef` _returnvalue))
      (`UserWidget.AddToViewport` _returnvalue 0)
      (`UserWidget.AddToViewport` _output_get 0)
      (set `/Game/UI/Dialog.TexArray` (`self.DoorText`) (`self.DialogUIRef`))
      (`KismetSystemLibrary.Delay` 2.0)
      (`self.Reset Dialog`))))

(event `Reset Dialog`
  (goto _label :!via `Reset`))

(fn `UserConstructionScript`)