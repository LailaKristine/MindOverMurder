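; Right-hand swinging door that opens for the player or listed AI and also teleports the player across it.
; Box overlaps play and reverse a yaw timeline, tracking one occupant via a busy flag, with open/close sounds for the player.
; Tick toggles door collision from the rotation, briefly disabling it when fully open.
; Two side triggers move the player to the opposite marker mesh behind a temporary black-screen widget with input disabled.
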(event `self.ReceiveTick`
  (params (DeltaSeconds :type "Float (single-precision)"))
  ;[1 1 1] Rotate door/playing door sound
  (if (== (stale `self.Box.OnComponentBeginOverlap` _doorrotation) 0.0)
    (`PrimitiveComponent.SetCollisionEnabled` (`self.Door`) "QueryAndPhysics")
    (elif (== 90.0 (stale `self.Box.OnComponentBeginOverlap` _doorrotation))
      (`PrimitiveComponent.SetCollisionEnabled` (`self.Door`) "NoCollision")
      (`KismetSystemLibrary.Delay` 2.0)
      (`PrimitiveComponent.SetCollisionEnabled` (`self.Door`) "QueryAndPhysics"))))

(event `self.Box.OnComponentBeginOverlap`
  (params (OverlappedComponent :type "PrimitiveComponent Object Reference") (OtherActor :type "Actor Object Reference") (OtherComp :type "PrimitiveComponent Object Reference") (OtherBodyIndex :type Integer) (bFromSweep :type Boolean) (SweepResult :type "HitResult Structure (by ref)"))
  (bind _returnvalue (`GameplayStatics.GetPlayerPawn` 0))
  ;[1 1 1] Rotate door/playing door sound
  (`|ExecutionSequence`
    (:`then_0`
      (goto _label_2 :!via `Reset`))
    (:`then_1`
      (if (`self.DoorBusy`)
        _
        (elif (== OtherActor _returnvalue)
          (set `self.ActorPointer` _returnvalue)
          (set `self.DoorBusy` true)
          (`|ExecutionSequence`
            (:`then_0`
              (bind (_direction _doorrotation) (`Timeline|DoorTimeline` :!label _label)
                (:`Update`
                  (`SceneComponent.K2_SetRelativeRotation` (`self.Door`) (`KismetMathLibrary.MakeRotator` 0.0 0.0 _doorrotation) false false))))
            (:`then_1`
              (`/Engine/EditorBlueprintResources/StandardMacros.DoOnce` false :!label _label_2
                (:`Completed`
                  (`GameplayStatics.PlaySoundAtLocation` "/Game/Sound/OpenDoor2.OpenDoor2" (`self.K2_GetActorLocation`) (struct) 0.4 1.0 0.0 null null null)))))
          (else
            (for _array_element (`/Game/AI/AI_BP.AllChildren` (`self.AIRef`))
              (if (== OtherActor _array_element)
                (set `self.ActorPointer` _array_element)
                (set `self.DoorBusy` true)
                (goto _label)))))))))

(event `self.Box.OnComponentEndOverlap`
  (params (OverlappedComponent :type "PrimitiveComponent Object Reference") (OtherActor :type "Actor Object Reference") (OtherComp :type "PrimitiveComponent Object Reference") (OtherBodyIndex :type Integer))
  (bind _actorpointer (`self.ActorPointer`))
  ;[1 1 1] Rotate door/playing door sound
  (`|ExecutionSequence`
    (:`then_0`
      (goto _label_3 :!via `Reset`))
    (:`then_1`
      (if (== OtherActor _actorpointer)
        (if (== _actorpointer (`GameplayStatics.GetPlayerPawn` 0))
          (set `self.DoorBusy` false)
          (`|ExecutionSequence`
            (:`then_0`
              (goto _label :!via `Reverse`))
            (:`then_1`
              (`KismetSystemLibrary.Delay` 1.0)
              (`/Engine/EditorBlueprintResources/StandardMacros.DoOnce` false :!label _label_3
                (:`Completed`
                  (`GameplayStatics.PlaySoundAtLocation` "/Game/Sound/CloseDoor3.CloseDoor3" (`self.K2_GetActorLocation`) (struct) 0.4 1.0 0.0 null null null)))))
          (else
            (set `self.DoorBusy` false)
            (goto _label :!via `Reverse`)))))))

(event `self.PBox-A.OnComponentBeginOverlap`
  (params (OverlappedComponent :type "PrimitiveComponent Object Reference") (OtherActor :type "Actor Object Reference") (OtherComp :type "PrimitiveComponent Object Reference") (OtherBodyIndex :type Integer) (bFromSweep :type Boolean) (SweepResult :type "HitResult Structure (by ref)"))
  (bind _returnvalue (`GameplayStatics.GetPlayerPawn` 0))
  ;[1 1 1] Teleports Player through door
  (if (== OtherActor _returnvalue)
    (`self.DisableInput` _returnvalue null)
    (bind _returnvalue_2 (`|CreateWidget` "/Game/UI/BlackScreen.BlackScreen_C"))
    (bind _output_get (set `self.BlackScreenRef` _returnvalue_2))
    (`UserWidget.AddToViewport` _output_get 0)
    (`KismetSystemLibrary.Delay` 0.5)
    (`self.K2_SetActorLocation` _returnvalue (`SceneComponent.K2_GetComponentLocation` (`self.StaticMeshB`)) false true)
    (`KismetSystemLibrary.Delay` 0.5)
    (`Widget.RemoveFromParent` _output_get)
    (`self.EnableInput` _returnvalue null)))

(event `self.PBox-B.OnComponentBeginOverlap`
  (params (OverlappedComponent :type "PrimitiveComponent Object Reference") (OtherActor :type "Actor Object Reference") (OtherComp :type "PrimitiveComponent Object Reference") (OtherBodyIndex :type Integer) (bFromSweep :type Boolean) (SweepResult :type "HitResult Structure (by ref)"))
  (bind _returnvalue (`GameplayStatics.GetPlayerPawn` 0))
  ;[1 1 1] Teleports Player through door
  (if (== OtherActor _returnvalue)
    (`self.DisableInput` _returnvalue null)
    (bind _returnvalue_2 (`|CreateWidget` "/Game/UI/BlackScreen.BlackScreen_C"))
    (bind _output_get (set `self.BlackScreenRef` _returnvalue_2))
    (`UserWidget.AddToViewport` _output_get 0)
    (`KismetSystemLibrary.Delay` 0.5)
    (`self.K2_SetActorLocation` _returnvalue (`SceneComponent.K2_GetComponentLocation` (`self.StaticMeshA`)) false true)
    (`KismetSystemLibrary.Delay` 0.5)
    (`Widget.RemoveFromParent` _output_get)
    (`self.EnableInput` _returnvalue null)))

(fn `UserConstructionScript`)