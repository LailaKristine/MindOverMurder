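; Camera actor that can turn to face the player pawn from its own position and shares its heading with the player.
; When FollowPlayer is enabled, each tick rotates the actor along the vector toward the player pawn without changing its location.
; It then casts the pawn to MyPlayer_BP and writes the camera's yaw into that pawn's CamYaw.
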(event `self.ReceiveBeginPlay`)

(event `self.ReceiveTick`
  (params (DeltaSeconds :type "Float (single-precision)"))
  (if (`self.FollowPlayer?`)
    (`self.FollowPlayer`)))

(fn `FollowPlayer`
  (`self.K2_SetActorRotation` (`KismetMathLibrary.Conv_VectorToRotator` (- (`self.K2_GetActorLocation` (`GameplayStatics.GetPlayerPawn` 0)) (`self.K2_GetActorLocation`))))
  (`self.SetRefToCam`))

(fn `SetRefToCam`
  (bind (_returnvalue_roll _returnvalue_pitch _returnvalue_yaw) (`KismetMathLibrary.BreakRotator` (`self.K2_GetActorRotation`)))
  (bind _asmy_player_bp (cast `/Game/MyPlayer_BP` (`GameplayStatics.GetPlayerPawn` 0)))
  (set `/Game/MyPlayer_BP.CamYaw` _returnvalue_yaw _asmy_player_bp))

(fn `UserConstructionScript`)