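; HMDialog_BP is a one-shot trigger actor that shows dialog when the referenced HeadMistress actor enters its Box.
; The first matching overlap creates a Dialog widget, adds it to the viewport, then passes DialogText into its TexArray.
; When that actor leaves the Box, a three-second delay precedes removing the widget and destroying the trigger.
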(event `self.Box.OnComponentBeginOverlap`
  (params (OverlappedComponent :type "PrimitiveComponent Object Reference") (OtherActor :type "Actor Object Reference") (OtherComp :type "PrimitiveComponent Object Reference") (OtherBodyIndex :type Integer) (bFromSweep :type Boolean) (SweepResult :type "HitResult Structure (by ref)"))
  (if (== OtherActor (`self.HeadMistressRef`))
    (`/Engine/EditorBlueprintResources/StandardMacros.DoOnce` false
      (:`Completed`
        (bind _returnvalue (`|CreateWidget` "/Game/UI/Dialog.Dialog_C"))
        (bind _output_get (set `self.DialogUI` _returnvalue))
        (`UserWidget.AddToViewport` _output_get 0)
        (`/Engine/EditorBlueprintResources/StandardMacros.DoOnce` false
          (:`Completed`
            (set `/Game/UI/Dialog.TexArray` (`self.DialogText`) (`self.DialogUI`))))))))

(event `self.Box.OnComponentEndOverlap`
  (params (OverlappedComponent :type "PrimitiveComponent Object Reference") (OtherActor :type "Actor Object Reference") (OtherComp :type "PrimitiveComponent Object Reference") (OtherBodyIndex :type Integer))
  (if (== OtherActor (`self.HeadMistressRef`))
    (`KismetSystemLibrary.Delay` 3.0)
    (`Widget.RemoveFromParent` (`self.DialogUI`))
    (`self.K2_DestroyActor`)))

(fn `UserConstructionScript`)