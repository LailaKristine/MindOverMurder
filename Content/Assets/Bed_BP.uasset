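; Bed_BP is an interactable bed that restarts the game through GameInstance_BP when the player uses it.
; A Box trigger shows a TextRender prompt while MyPlayer_BP overlaps it and hides it on exit.
; The Use event confirms that player still overlaps the box, then calls Restart on the game instance.
; A direct OpenLevel node for Day_Cycle is left unconnected.
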(event `self.Box.OnComponentBeginOverlap`
  (params (OverlappedComponent :type "PrimitiveComponent Object Reference") (OtherActor :type "Actor Object Reference") (OtherComp :type "PrimitiveComponent Object Reference") (OtherBodyIndex :type Integer) (bFromSweep :type Boolean) (SweepResult :type "HitResult Structure (by ref)"))
  (bind _asmy_player_bp (cast `/Game/MyPlayer_BP` OtherActor))
  (`SceneComponent.SetVisibility` (`self.TextRender`) true false))

(event `self.Box.OnComponentEndOverlap`
  (params (OverlappedComponent :type "PrimitiveComponent Object Reference") (OtherActor :type "Actor Object Reference") (OtherComp :type "PrimitiveComponent Object Reference") (OtherBodyIndex :type Integer))
  (cast `/Game/MyPlayer_BP` OtherActor)
  (`SceneComponent.SetVisibility` (`self.TextRender`) false false))

(event `/Game/Items/Use.Use`
  (if (`PrimitiveComponent.IsOverlappingActor` (`self.Box`) (stale `self.Box.OnComponentBeginOverlap` _asmy_player_bp))
    (bind _asgame_instance_bp (cast `/Game/GameInstance_BP` (`GameplayStatics.GetGameInstance`)))
    (`/Game/GameInstance_BP.Restart` _asgame_instance_bp)))

(fn `UserConstructionScript`)