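; Broken heater that the player must fix before rising cold kills them.
; Tick ramps a coldness filter's blend weight over two minutes, calls the empty KillJanitor stub once at the halfway mark, then triggers player death.
; Use marks it fixed, destroys heater and player particles and hides AI children's cold breath; Tick then clears the filter once.
; Without a valid filter, BeginPlay disables Tick.
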(event `self.ReceiveBeginPlay`
  (bind _coldnessfilterptr (`self.ColdnessFilterPtr`))
  (`/Engine/EditorBlueprintResources/StandardMacros.IsValid` _coldnessfilterptr
    (:`Is Valid`
      (set `PostProcessVolume.BlendWeight` 0.0 _coldnessfilterptr :!label _label))
    (:`Is Not Valid`
      (`self.SetActorTickEnabled` false))))

(event `self.ReceiveTick`
  (params (DeltaSeconds :type "Float (single-precision)"))
  (bind _coldnessfilterptr (`self.ColdnessFilterPtr`))
  (if (`self.IsFixed`)
    (`/Engine/EditorBlueprintResources/StandardMacros.DoOnce` false
      (:`Completed`
        (goto _label)))
    (elif (< (`self.SecondsElapsed`) 120.0)
      (bind _output_get (set `self.SecondsElapsed` (+ (`self.SecondsElapsed`) DeltaSeconds)))
      (`/Engine/EditorBlueprintResources/StandardMacros.IsValid` _coldnessfilterptr
        (:`Is Valid`
          (set `PostProcessVolume.BlendWeight` (* _output_get 0.008333) _coldnessfilterptr)
          (if (not (< (`self.SecondsElapsed`) 60.0))
            (`/Engine/EditorBlueprintResources/StandardMacros.DoOnce` false
              (:`Completed`
                (`self.KillJanitor`))))))
      (else
        (`/Engine/EditorBlueprintResources/StandardMacros.DoOnce` false
          (:`Completed`
            (bind _asmy_player_bp (cast `/Game/MyPlayer_BP` (`GameplayStatics.GetPlayerPawn` 0)))
            (`/Game/MyPlayer_BP.Death` _asmy_player_bp 4)))))))

(event `/Game/Items/Use.Use`
  (if (not (`self.IsFixed`))
    (`ActorComponent.K2_DestroyComponent` (`self.ParticleSystem`))
    (bind _asmy_player_bp (cast `/Game/MyPlayer_BP` (`GameplayStatics.GetPlayerPawn` 0)))
    (`ActorComponent.K2_DestroyComponent` (`/Game/MyPlayer_BP.ParticleSystem` _asmy_player_bp))
    (set `self.IsFixed` true)
    (for _array_element (`/Game/AI/AI_BP.AllChildren` (`self.AIPtr`))
      (`SceneComponent.SetVisibility` (`/Game/AI/AI_BP.ColdBreath` _array_element) false false))))

(fn `KillJanitor`)

(fn `UserConstructionScript`)